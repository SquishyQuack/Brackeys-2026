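; BP_Opponent is the AI rival in a revolver duel, a traffic light mesh with hit points and an action counter.
; After picking up the shared BP_Revolver, it waits a random delay, then randomly either shoots, spending an action, or turns the revolver and decides again.
; Damage updates its health widget and plays a cue; at zero health the mesh switches to physics and is launched backward and upward.
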(event `/Game/Brackeys2026/Interfaces/BPI_Action.AddAction`
  (`/Engine/EditorBlueprintResources/StandardMacros.IncrementInt` (`self.Actions`)))

(event `self.ReceiveBeginPlay`
  (bind _returnvalue (`GameplayStatics.GetActorOfClass` "/Game/Brackeys2026/Objects/Revolver/BP_Revolver.BP_Revolver_C"))
  (set `self.RevolverReference` _returnvalue)
  (bind _returnvalue_2 (`|CreateWidget` "/Game/Brackeys2026/UI/BP_UIOpponent.BP_UIOpponent_C" (`GameplayStatics.GetPlayerController` 0)))
  (set `self.EnemyUI` _returnvalue_2))

(event `self.ReceiveAnyDamage`
  (params (Damage :type "Float (single-precision)") (DamageType :type "DamageType Object Reference") (InstigatedBy :type "Controller Object Reference") (DamageCauser :type "Actor Object Reference"))
  (bind _trafficlight3_low_poly (`self.trafficlight3_low_poly`))
  (bind _output_get (set `self.HitPoints` (- (`self.HitPoints`) Damage)))
  (`/Game/Brackeys2026/UI/BP_UIOpponent.SetEnemyHealth` (`self.EnemyUI`) _output_get)
  (`AudioComponent.Play` (`self.BP_CueOpponent`) 0.0)
  (if (== _output_get 0.0)
    (`KismetSystemLibrary.Delay` 0.3)
    (`PrimitiveComponent.SetSimulatePhysics` _trafficlight3_low_poly true)
    (`PrimitiveComponent.AddImpulse` _trafficlight3_low_poly (+ (* (`self.GetActorForwardVector`) -200000) (* (`self.GetActorUpVector`) 200000)) "None" false)
    (`KismetSystemLibrary.Delay` 4.0)))

(event `PickUpGun`
  (`KismetSystemLibrary.Delay` 1.5)
  (`/Game/Brackeys2026/Objects/Revolver/BP_Revolver.PickUpGun` (`self.RevolverReference`) (`self.RevovlerPosition`))
  (`KismetSystemLibrary.Delay` (`KismetMathLibrary.RandomFloatInRange` 2.0 4.0))
  (`self.DecideAction`))

(event `DecideAction`
  (bind _revolverreference (`self.RevolverReference`))
  (if (`KismetMathLibrary.RandomBool`)
    (`/Game/Brackeys2026/Objects/Revolver/BP_Revolver.Shoot` _revolverreference)
    (`/Engine/EditorBlueprintResources/StandardMacros.DecrementInt` (`self.Actions`))
    (else
      (`/Game/Brackeys2026/Objects/Revolver/BP_Revolver.TurnRevolver` _revolverreference)
      (`KismetSystemLibrary.Delay` (`KismetMathLibrary.RandomFloatInRange` 1.5 2.5))
      (`self.DecideAction`))))

(fn `UserConstructionScript`)