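; BP_Revolver is a clickable revolver that the player picks up, fires once and puts back down.
; Timelines lerp it between its original transform and the player's RevolverPosition, with firing automatic after a delay.
; LoadBullets queues six random live or blank rounds, and each shot consumes the first while flashing a light.
; Live rounds damage BPI_Action actors via line trace; blanks use a short trace, granting an action message when aimed at the holder.
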(event `self.ReceiveBeginPlay`
  ;[1 1 1] Get references and set original transform
  (set `self.OriginalTransform` (`self.GetTransform`))
  (bind _returnvalue (`GameplayStatics.GetActorOfClass` "/Game/Brackeys2026/Characters/Player/BP_Player.BP_Player_C"))
  (set `self.PlayerReference` _returnvalue)
  (bind _returnvalue_2 (`GameplayStatics.GetActorOfClass` "/Game/Brackeys2026/Characters/Opponent/BP_Opponent.BP_Opponent_C"))
  (set `self.OpponentReference` _returnvalue_2)
  (bind _returnvalue_3 (`GameplayStatics.GetActorOfClass` "/Game/Brackeys2026/Objects/Phone/BP_Phone.BP_Phone_C"))
  (set `self.PhoneReference` _returnvalue_3))

(event `self.Revolver.OnClicked`
  (params (TouchedComponent :type "PrimitiveComponent Object Reference") (ButtonPressed :type "Key Structure"))
  (bind (_originaltransform_location _originaltransform_rotation _originaltransform_scale) (`KismetMathLibrary.BreakTransform` (`self.OriginalTransform`)))
  (bind (_returnvalue_location _returnvalue_rotation) (`KismetMathLibrary.BreakTransform` (`SceneComponent.K2_GetComponentToWorld` (`/Game/Brackeys2026/Characters/Player/BP_Player.RevolverPosition` (`self.PlayerReference`)))))
  (bind (_direction _alpha) (`Timeline|PickUpTimeline` :!via `PlayFromStart`)
    (:`Update`
      (`self.K2_SetActorTransform` (`KismetMathLibrary.TLerp` (`self.OriginalTransform`) (`KismetMathLibrary.MakeTransform` _returnvalue_location _returnvalue_rotation _originaltransform_scale) _alpha)))
    (:`Finished`
      (set `/Game/Brackeys2026/Characters/Player/BP_Player.HoldingRevolver` true (`self.PlayerReference`))
      (`KismetSystemLibrary.Delay` 1.0)
      (`self.Shoot`)
      (`KismetSystemLibrary.Delay` 1.0)
      (`self.PutDownRevolver`))))

(event `Shoot`
  (bind _returnvalue (`self.K2_GetActorLocation`))
  (bind _returnvalue_2 (`self.K2_GetActorLocation`))
  ;[1 1 1] Shoot confiuration
  (`LightComponent.SetIntensity` (`self.PointLight`) 10000.0)
  (if (`|GetArrayItem` (`self.IsLiveBullet`))
    ;;[1 1 1] Fire bullet and apply damage with live bullet
    (bind _outhit (`KismetSystemLibrary.LineTraceSingle` _returnvalue (+ _returnvalue (* (`self.GetActorForwardVector`) 4000)) "TraceTypeQuery1"))
    (bind (_bblockinghit _binitialoverlap _time _distance _location _impactpoint _normal _impactnormal _physmat _hitactor) (`GameplayStatics.BreakHitResult` _outhit))
    (if (`KismetSystemLibrary.DoesImplementInterface` _hitactor "/Game/Brackeys2026/Interfaces/BPI_Action.BPI_Action_C")
      (`GameplayStatics.ApplyDamage` _hitactor 1.0))
    (else
      ;;[1 1 1] Add action if revolver is turned towards character holding it
      (bind _outhit_2 (`KismetSystemLibrary.LineTraceSingle` _returnvalue_2 (+ _returnvalue_2 (* (`self.GetActorForwardVector`) 100)) "TraceTypeQuery1"))
      (bind (_bblockinghit_2 _binitialoverlap_2 _time_2 _distance_2 _location_2 _impactpoint_2 _normal_2 _impactnormal_2 _physmat_2 _hitactor_2) (`GameplayStatics.BreakHitResult` _outhit_2))
      (if (`KismetSystemLibrary.DoesImplementInterface` _hitactor_2 "/Game/Brackeys2026/Interfaces/BPI_Action.BPI_Action_C")
        (message `/Game/Brackeys2026/Interfaces/BPI_Action.AddAction` _hitactor_2))))
  (`KismetArrayLibrary.Array_Remove` (`self.IsLiveBullet`))
  (`/Engine/EditorBlueprintResources/StandardMacros.DecrementInt` (`self.BulletsRemaining`)
    (:`  `
      (`KismetSystemLibrary.Delay` 0.2)
      (`LightComponent.SetIntensity` (`self.PointLight`) 0.0))))

(event `PutDownRevolver`
  (bind (_direction _alpha) (`Timeline|PutDownTimeline` :!via `PlayFromStart`)
    (:`Update`
      (`self.K2_SetActorTransform` (`KismetMathLibrary.TLerp` (`self.GetTransform`) (`self.OriginalTransform`) _alpha)))
    (:`Finished`
      (set `/Game/Brackeys2026/Characters/Player/BP_Player.HoldingRevolver` false (`self.PlayerReference`)))))

(fn `LoadBullets`
  (for _ (range 6)
    (`KismetArrayLibrary.Array_Add` (`self.IsLiveBullet`) (`KismetMathLibrary.RandomBool`)))
  (set `self.BulletsRemaining` 6)
  (return))

(fn `UserConstructionScript`)