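; BP_Revolver is the shared revolver in a turn-based, Russian roulette-style game between player and opponent.
; Clicking it starts a timeline pickup to the player's hand; TurnRevolver rotates it half a turn.
; Shoot consumes the shuffled chamber's first round, line-tracing for BPI_Action pawns to damage when live or message when blank.
; It then returns to rest, reloads through a C++ LoadBullets function when empty, and calls the GameMode's TurnCheck.
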(event `self.ReceiveBeginPlay`
  ;[1 1 1] Get references and set original transform
  (bind _returnvalue (`GameplayStatics.GetActorOfClass` "/Game/Brackeys2026/Characters/Player/BP_Player.BP_Player_C"))
  (set `self.PlayerReference` _returnvalue)
  (bind _asbrackeys_game_mode (cast `/Game/Brackeys2026/Levels/BrackeysGameMode` (`GameplayStatics.GetGameMode`)))
  (set `self.GameModeReference` _asbrackeys_game_mode)
  (bind _returnvalue_2 (`GameplayStatics.GetActorOfClass` "/Game/Brackeys2026/Characters/Opponent/BP_Opponent.BP_Opponent_C"))
  (set `self.OpponentReference` _returnvalue_2)
  (bind _returnvalue_3 (`GameplayStatics.GetActorOfClass` "/Game/Brackeys2026/Objects/Phone/BP_Phone.BP_Phone_C"))
  (set `self.PhoneReference` _returnvalue_3)
  (set `self.OriginalTransform` (`self.GetTransform`))
  (`KismetSystemLibrary.Delay` 12.75)
  (`self.LoadBullets`))

(event `self.Revolver_separated_Revolver.OnClicked`
  (params (TouchedComponent :type "PrimitiveComponent Object Reference") (ButtonPressed :type "Key Structure"))
  (`PrimitiveComponent.SetCollisionEnabled` (`self.Revolver_separated_Revolver`) "NoCollision")
  (`self.PickUpGun` (`/Game/Brackeys2026/Characters/Player/BP_Player.RevolverPosition` (`self.PlayerReference`))))

(event `PickUpGun`
  (params (RevolverPosition :type "SceneComponent Object Reference"))
  (bind (_returnvalue_location _returnvalue_rotation) (`KismetMathLibrary.BreakTransform` (`SceneComponent.K2_GetComponentToWorld` RevolverPosition)))
  (bind _bp_cuerevolver (`self.BP_CueRevolver`))
  (bind (_originaltransform_location _originaltransform_rotation _originaltransform_scale) (`KismetMathLibrary.BreakTransform` (`self.OriginalTransform`)))
  (set `/Game/Brackeys2026/Objects/Phone/BP_Phone.IsPhoneOn` false (`self.PhoneReference`))
  (`AudioComponent.SetIntParameter` _bp_cuerevolver "SoundEffect" 2)
  (`AudioComponent.Play` _bp_cuerevolver 0.0)
  (bind (_direction _alpha) (`Timeline|PickUpTimeline` :!via `PlayFromStart`)
    (:`Update`
      (`self.K2_SetActorTransform` (`KismetMathLibrary.TLerp` (`self.OriginalTransform`) (`KismetMathLibrary.MakeTransform` _returnvalue_location _returnvalue_rotation _originaltransform_scale) _alpha)))
    (:`Finished`
      (if (`/Game/Brackeys2026/Levels/BrackeysGameMode.IsPlayerTurn` (`self.GameModeReference`))
        (`/Game/Brackeys2026/Characters/Player/BP_Player.SetHoldingRevolver` (`self.PlayerReference`) true)))))

(event `Shoot`
  (bind (_chamberoriginalrotation_roll _chamberoriginalrotation_pitch _chamberoriginalrotation_yaw) (`KismetMathLibrary.BreakRotator` (`self.ChamberOriginalRotation`)))
  (bind _bp_cuerevolver (`self.BP_CueRevolver`))
  (bind (_relativerotation_roll _relativerotation_pitch _relativerotation_yaw) (`KismetMathLibrary.BreakRotator` (`SceneComponent.RelativeRotation` (`self.Revolver_Hammer`))))
  (`/Game/Brackeys2026/Objects/Phone/BP_Phone.HideAllHint` (`self.PhoneReference`))
  (`KismetSystemLibrary.Delay` 1.5)
  (if (`|GetArrayItem` (`self.IsLiveBullet`))
    ;[1 1 1] Live bullet line trace
    (`LightComponent.SetIntensity` (`self.PointLight`) 10000.0)
    (bind (_hitactor _doesimplementinterface) (`self.RevolverLineTrace` 4000))
    (if _doesimplementinterface
      (set `self.WaitTime` 5.0)
      (`GameplayStatics.ApplyDamage` _hitactor 1.0))
    (else
      ;[1 1 1] No bullet line trace
      (bind (_hitactor_2 _doesimplementinterface_2) (`self.RevolverLineTrace` 100))
      (`AudioComponent.SetIntParameter` _bp_cuerevolver "SoundEffect" 1)
      (`AudioComponent.Play` _bp_cuerevolver 0.0)
      (set `self.WaitTime` 1.5)
      (if _doesimplementinterface_2
        (message `/Game/Brackeys2026/Interfaces/BPI_Action.AddAction` _hitactor_2))))
  (`KismetArrayLibrary.Array_Remove` (`self.IsLiveBullet`))
  (`/Engine/EditorBlueprintResources/StandardMacros.DecrementInt` (`self.BulletsRemaining`)
    (:`  `
      (set `self.HammerOriginalRotation` (`SceneComponent.RelativeRotation` (`self.Revolver_Hammer`)))
      (set `self.ChamberOriginalRotation` (`SceneComponent.RelativeRotation` (`self.Revolver_Chamber`)))
      ;[1 1 1] Revolver Animation
      (bind (_direction _hammeralpha _chamberalpha) (`Timeline|RevolverTimeline` :!via `PlayFromStart`)
        (:`Update`
          (`SceneComponent.K2_SetRelativeRotation` (`self.Revolver_Hammer`) (`KismetMathLibrary.RLerp` (`self.HammerOriginalRotation`) (`KismetMathLibrary.MakeRotator` (+ _relativerotation_roll 10.0) _relativerotation_pitch _relativerotation_yaw) _hammeralpha) false false)
          (`SceneComponent.K2_SetRelativeRotation` (`self.Revolver_Chamber`) (`KismetMathLibrary.RLerp` (`self.ChamberOriginalRotation`) (`KismetMathLibrary.MakeRotator` _chamberoriginalrotation_roll (- _chamberoriginalrotation_pitch 60.0) _chamberoriginalrotation_yaw) _chamberalpha) false false))
        (:`Finished`
          (`KismetSystemLibrary.Delay` 0.2)
          (`LightComponent.SetIntensity` (`self.PointLight`) 0.0)
          (`KismetSystemLibrary.Delay` (`self.WaitTime`))
          (`self.PutDownRevolver`))))))

(event `TurnRevolver`
  (bind (_revolveroriginalrotaion_roll _revolveroriginalrotaion_pitch _revolveroriginalrotaion_yaw) (`KismetMathLibrary.BreakRotator` (`self.RevolverOriginalRotaion`)))
  (set `self.RevolverOriginalRotaion` (`self.K2_GetActorRotation`))
  (bind (_direction _turnalpha) (`Timeline|TurnTimeline` :!via `PlayFromStart`)
    (:`Update`
      (`self.K2_SetActorRotation` (`KismetMathLibrary.RLerp` (`self.RevolverOriginalRotaion`) (`KismetMathLibrary.MakeRotator` _revolveroriginalrotaion_roll _revolveroriginalrotaion_pitch (+ _revolveroriginalrotaion_yaw 180.0)) _turnalpha)))))

(event `Reload`
  (bind _originaltransform_location (`KismetMathLibrary.BreakTransform` (`self.OriginalTransform`)))
  (bind (_originaltransform_location_2 _originaltransform_rotation) (`KismetMathLibrary.BreakTransform` (`self.OriginalTransform`)))
  (bind (_direction _position) (`Timeline|StartReloadTimline` :!via `PlayFromStart`)
    (:`Update`
      (`self.K2_SetActorLocation` (`KismetMathLibrary.VLerp` (`self.K2_GetActorLocation`) (+ _originaltransform_location (* (`self.GetActorForwardVector`) 1000)) _position)))
    (:`Finished`
      (`self.LoadBullets`)
      (`KismetSystemLibrary.Delay` 1.0)
      (bind (_direction_2 _position_2 _rotation) (`Timeline|EndReloadTimeline` :!via `PlayFromStart`)
        (:`Update`
          (`self.K2_SetActorLocation` (`KismetMathLibrary.VLerp` (`self.K2_GetActorLocation`) _originaltransform_location_2 _position_2)))))))

(event `PutDownRevolver`
  (bind _bp_cuerevolver (`self.BP_CueRevolver`))
  (`AudioComponent.SetIntParameter` _bp_cuerevolver "SoundEffect" 3)
  (`AudioComponent.Play` _bp_cuerevolver 0.0)
  (bind (_direction _alpha) (`Timeline|PutDownTimeline` :!via `PlayFromStart`)
    (:`Update`
      (`self.K2_SetActorTransform` (`KismetMathLibrary.TLerp` (`self.GetTransform`) (`self.OriginalTransform`) _alpha)))
    (:`Finished`
      (if (== (`self.BulletsRemaining`) 0)
        (`self.Reload`)
        (`KismetSystemLibrary.Delay` 3.0))
      (set `/Game/Brackeys2026/Characters/Player/BP_Player.HoldingRevolver` false (`self.PlayerReference`))
      (`PrimitiveComponent.SetCollisionEnabled` (`self.Revolver_separated_Revolver`) "QueryAndPhysics")
      (`/Game/Brackeys2026/Levels/BrackeysGameMode.TurnCheck` (`self.GameModeReference`)))))

(fn `LoadBullets`
  (locals (MaxLiveBullets :type Integer))
  (bind _bp_cuerevolver (`self.BP_CueRevolver`))
  (bind (_bulletschamber _maxlivebullets _bulletsremaining) (`RevolverBlueprintLib.LoadBullets`)) ; Above loadBullets function written to a C++ Funcion of RevolverBlueprintLib.cpp - to improve perfomance in game
  (set `self.BulletsRemaining` _bulletsremaining)
  (set `local.MaxLiveBullets` _maxlivebullets)
  (set `self.IsLiveBullet` _bulletschamber)
  (`AudioComponent.SetIntParameter` _bp_cuerevolver "SoundEffect" 0)
  (`AudioComponent.Play` _bp_cuerevolver 0.0)
  (`KismetArrayLibrary.Array_Shuffle` (`self.IsLiveBullet`))
  (return))

(fn `UserConstructionScript`)